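; Base pickup actor that homes in on the player and awards points when collected.
; Overlapping the outer Trigger with the player plays a sound and starts a timeline, used as a temporary tick, that moves the pickup via VInterpTo toward the player's current position.
; Overlap of SphereColliderDestroy with the PC adds PointValue to its points and destroys the pickup.
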(event `self.trigger.OnComponentBeginOverlap`
  (params (OverlappedComponent :type "PrimitiveComponent Object Reference") (OtherActor :type "Actor Object Reference") (OtherComp :type "PrimitiveComponent Object Reference") (OtherBodyIndex :type Integer) (bFromSweep :type Boolean) (SweepResult :type "HitResult Structure (by ref)"))
  ;[1 1 1] Lerp towards player
  (bind _result (`/Game/Roncin/BlueprintFunctionLibrary/MyBPFunctions.ConfirmOtherActorIsPlayer` OtherActor))
  (if _result
    (`GameplayStatics.SpawnSoundAtLocation` "/Game/Roncin/Pickup/wah_wah3.wah_wah3" (`self.K2_GetActorLocation`) (struct) 1.0 1.0 0.0 null null)
    ;;[1 1 1] Vinterpret towards player.
    (bind (_direction _newtrack_0) (`Timeline|Timeline_1` :!via `PlayFromStart`)
      (:`Update`
        (`self.K2_SetActorLocation` (+ _newtrack_0 (`KismetMathLibrary.VInterpTo` (`self.K2_GetActorLocation`) (`self.K2_GetActorLocation` (`GameplayStatics.GetPlayerCharacter` 0)) (`GameplayStatics.GetWorldDeltaSeconds`) (`self.Interp Speed`))))))))

(event `self.SphereCollider - destroy.OnComponentBeginOverlap`
  (params (OverlappedComponent :type "PrimitiveComponent Object Reference") (OtherActor :type "Actor Object Reference") (OtherComp :type "PrimitiveComponent Object Reference") (OtherBodyIndex :type Integer) (bFromSweep :type Boolean) (SweepResult :type "HitResult Structure (by ref)"))
  ;[1 1 1] apply effects on hit.
  (bind _aspc (cast `/Game/ThirdPersonBP/Blueprints/PC` OtherActor))
  (`/Game/ThirdPersonBP/Blueprints/PC.IncrementPoints` _aspc (`self.PointValue`))
  (`self.K2_DestroyActor`)
  (`KismetSystemLibrary.PrintString` "pickup destroyed"))

(fn `UserConstructionScript`)